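; Enemy Gameplay Ability for a ranged attack that fires a projectile at the avatar's combat target.
; On activation it gets the target through the Combat Interface, turns to face it and plays a random tagged attack montage.
; A gameplay event matching that montage's tag triggers SpawnProjectile toward the target's current location.
; The ability ends when the montage completes, is interrupted or is cancelled.
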(event Ability|EventActivateAbility
  (bind _returnvalue (Ability|GetAvatarActorfromActorInfo))
  ;[0.15 0.15 0.15 0.5] Get the Combat Interface of the Actor and face the target
  (bind _returnvalue_2 (Class|EnemyInterface|GetCombatTarget(Message) _returnvalue))
  (bind _output_get (Variables|Default|SetCombatTarget _returnvalue_2))
  (bind _ascombat_interface (Utilities|Casting|CastToCombatInterface _returnvalue))
  (Class|CombatInterface|UpdateFacingTarget _ascombat_interface (Transformation|GetActorLocation _output_get))
  ;[0.15 0.15 0.15 0.5] Get one of the Attack Montages to play and its associated Tag to listen for on attack
  (bind _returnvalue_3 (Class|CombatInterface|GetAttackMontages(Message) (Ability|GetAvatarActorfromActorInfo)))
  (bind _output_get_2 (Variables|Default|SetTaggedMontage (Class|AuraDamageGameplayAbility|GetRandomTaggedMontage _returnvalue_3)))
  (|PlayMontageandWaitProxy "None" (.MontageAsset (Utilities|Struct|BreakTaggedMontage _output_get_2)) 1.0 "None" true 1.0 0.0 false
    (:then
      (Ability|Tasks|WaitGameplayEvent (.MontageTag (Utilities|Struct|BreakTaggedMontage _output_get_2)) 0
        (:EventReceived
          (Class|CombatInterface|GetCombatSocketLocation(Message) (Ability|GetAvatarActorfromActorInfo) (.MontageTag (Utilities|Struct|BreakTaggedMontage _output_get_2)))
          (Class|AuraProjectileSpell|SpawnProjectile (Transformation|GetActorLocation (Variables|Default|GetCombatTarget))))))
    (:OnCompleted
      (Ability|EndAbility :!label _label))
    (:OnInterrupted
      (goto _label))
    (:OnCancelled
      (goto _label))))

(event Ability|EventOnEndAbility
  (params (bWasCancelled :type Boolean)))